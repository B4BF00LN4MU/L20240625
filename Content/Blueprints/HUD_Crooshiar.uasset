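; HUD Blueprint that draws a red, four-line crosshair around the screen center, intended to spread with the player character's movement speed.
; Each DrawHUD sets CrosshairOpen to velocity over max movement speed, scaled by CrosshairSize.
; Right and bottom lines draw before that update; left and top draw after it, only for a possessed Character.
; Left and top start points subtract center from opening, reversing the expected offset.
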(event EventDrawHUD
  (params (SizeX :type Integer) (SizeY :type Integer))
  (Variables|Default|SetCenterX (/ SizeX 2))
  (Variables|Default|SetCneterY (/ SizeY 2))
  ;[1 1 1] 십자가 오른쪽
  (Class|HUD|DrawLine (+ (Variables|Default|GetCrosshairOpen) (Variables|Default|GetCenterX)) (Math|Conversions|ToFloat(Integer) (Variables|Default|GetCneterY)) (+ (Variables|Default|GetCenterX) (Variables|Default|GetCrosshairSize) (Variables|Default|GetCrosshairOpen)) (Math|Conversions|ToFloat(Integer) (Variables|Default|GetCneterY)) "(R=1.000000,G=0.000000,B=0.000000,A=1.000000)" 1e+01)
  ;[1 1 1] 십자가 아래쪽
  (Class|HUD|DrawLine (Math|Conversions|ToFloat(Integer) (Variables|Default|GetCenterX)) (+ (Variables|Default|GetCrosshairOpen) (Variables|Default|GetCneterY)) (Math|Conversions|ToFloat(Integer) (Variables|Default|GetCenterX)) (+ (Variables|Default|GetCneterY) (Variables|Default|GetCrosshairSize) (Variables|Default|GetCrosshairOpen)) "(R=1.000000,G=0.000000,B=0.000000,A=1.000000)" 1e+01)
  (bind _ascharacter (Utilities|Casting|CastToCharacter (Pawn|GetControlledPawn (Game|GetPlayerController 0))))
  ;[1 1 1] 떨어진 거리 구하기
  (Variables|Default|SetCrosshairOpen (* (/ (Math|Vector|VectorLength (Variables|/Script/Engine.MovementComponent|GetVelocity (Variables|/Script/Engine.Character|GetCharacterMovement _ascharacter))) (Class|MovementComponent|GetMaxSpeed (Variables|/Script/Engine.Character|GetCharacterMovement _ascharacter))) (Variables|Default|GetCrosshairSize)))
  ;[1 1 1] 십자가 왼쪽
  (Class|HUD|DrawLine (- (Variables|Default|GetCrosshairOpen) (Variables|Default|GetCenterX)) (Math|Conversions|ToFloat(Integer) (Variables|Default|GetCneterY)) (Utilities|Operators|Subtract (Variables|Default|GetCenterX) (Variables|Default|GetCrosshairSize) (Variables|Default|GetCrosshairOpen)) (Math|Conversions|ToFloat(Integer) (Variables|Default|GetCneterY)) "(R=1.000000,G=0.000000,B=0.000000,A=1.000000)" 1e+01)
  ;[1 1 1] 십자가 위쪽
  (Class|HUD|DrawLine (Math|Conversions|ToFloat(Integer) (Variables|Default|GetCenterX)) (Math|Conversions|ToFloat(Integer) (- (Variables|Default|GetCrosshairOpen) (Variables|Default|GetCneterY))) (Math|Conversions|ToFloat(Integer) (Variables|Default|GetCenterX)) (Utilities|Operators|Subtract (Variables|Default|GetCneterY) (Variables|Default|GetCrosshairSize) (Variables|Default|GetCrosshairOpen)) "(R=1.000000,G=0.000000,B=0.000000,A=1.000000)" 1e+01))

(fn ConstructionScript)